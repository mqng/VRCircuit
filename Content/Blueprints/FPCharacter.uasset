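; First-person player character that looks, moves, and picks up physics objects tagged "Grabbable".
; A per-tick camera line trace highlights the targeted object through its "Selection Color" material parameter and clears the previous one.
; Grabbing traces again and holds the hit with a PhysicsHandle, first spawning a physics-simulated copy if it is tagged "IsOriginal".
; The Grabbing axis event keeps the handle target in front of the camera until release drops it.
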(event `self.ReceiveBeginPlay`)

(event `InputAxis|MouseX`
  (params (AxisValue :type "Float (single-precision)"))
  ;[1 1 1] Basic Movement Set
  (`self.AddControllerYawInput` AxisValue))

(event `InputAxis|MouseY`
  (params (AxisValue :type "Float (single-precision)"))
  ;[1 1 1] Basic Movement Set
  (`self.AddControllerPitchInput` AxisValue))

(event `InputAxis|MoveForward`
  (params (AxisValue :type "Float (single-precision)"))
  ;[1 1 1] Basic Movement Set
  (`self.AddMovementInput` (`self.GetActorForwardVector`) AxisValue))

(event `InputAxis|MoveRight`
  (params (AxisValue :type "Float (single-precision)"))
  ;[1 1 1] Basic Movement Set
  (`self.AddMovementInput` (`self.GetActorRightVector`) AxisValue))

(event `self.ReceiveTick`
  (params (DeltaSeconds :type "Float (single-precision)"))
  (bind _fpcamera (`self.FPCamera`))
  (bind _lastoverlapped (`self.LastOverlapped`))
  (bind _returnvalue (`SceneComponent.K2_GetComponentLocation` _fpcamera))
  (bind _returnvalue_2 (`KismetSystemLibrary.IsValidClass` (`GameplayStatics.GetObjectClass` _lastoverlapped)))
  ;[1 1 1] Highlighting of grabbable objects
  (bind _outhit (`KismetSystemLibrary.LineTraceSingle` :`Start` _returnvalue :`End` (+ _returnvalue (* (`SceneComponent.GetForwardVector` _fpcamera) 200.0)) :`TraceChannel` "TraceTypeQuery1" :`TraceColor` (struct :`R` 1.0 :`G` 1.0 :`B` 1.0 :`A` 1.0) :`TraceHitColor` (struct) :`DrawTime` 0.0))
  (bind (_bblockinghit _binitialoverlap _time _distance _location _impactpoint _normal _impactnormal _physmat _hitactor) (`GameplayStatics.BreakHitResult` _outhit))
  (if (`KismetSystemLibrary.IsValidClass` (`GameplayStatics.GetObjectClass` _hitactor))
    (if (`self.ActorHasTag` _hitactor "Grabbable")
      (set `self.NewOverlapped` _hitactor)
      (if (and (!= _lastoverlapped (`self.NewOverlapped`)) _returnvalue_2)
        (`MeshComponent.SetVectorParameterValueOnMaterials` (`self.GetComponentByClass` _lastoverlapped "/Script/Engine.StaticMeshComponent") "Selection Color" (0.0 0.0 0.0) :!label _label)
        (else
          (`MeshComponent.SetVectorParameterValueOnMaterials` (`self.GetComponentByClass` _hitactor "/Script/Engine.StaticMeshComponent") "Selection Color" (5.0 0.0 10.0))))
      (set `self.LastOverlapped` _hitactor)
      (elif _returnvalue_2
        (goto _label)))
    (elif _returnvalue_2
      (goto _label))))

(event `InputAction|Grabbing`
  (params (Key :type "Key Structure"))
  (bind _physicshandle (`self.PhysicsHandle`))
  (bind _fpcamera (`self.FPCamera`))
  (bind _returnvalue (`SceneComponent.K2_GetComponentLocation` _fpcamera))
  (bind _returnvalue_2 (`SceneComponent.GetForwardVector` _fpcamera))
  (:`Pressed`
    (bind (_outhit _returnvalue_3) (`KismetSystemLibrary.LineTraceSingle` :`Start` _returnvalue :`End` (+ _returnvalue (* _returnvalue_2 200.0)) :`TraceChannel` "TraceTypeQuery1" :`TraceColor` (struct :`R` 1.0 :`G` 1.0 :`B` 1.0 :`A` 1.0) :`TraceHitColor` (struct :`G` 1.0)))
    (if _returnvalue_3
      (bind (_bblockinghit _binitialoverlap _time _distance _location _impactpoint _normal _impactnormal _physmat _hitactor _hitcomponent) (`GameplayStatics.BreakHitResult` _outhit))
      (if (`self.ActorHasTag` _hitactor "Grabbable")
        (if (`ActorComponent.ComponentHasTag` (`self.GetComponentByClass` _hitactor "/Script/Engine.SceneComponent") "IsOriginal")
          (bind _returnvalue_4 (`SceneComponent.K2_GetComponentLocation` _hitcomponent))
          (bind _returnvalue_5 (`|SpawnActorFromClass` (`GameplayStatics.GetObjectClass` _hitactor) (`KismetMathLibrary.Conv_VectorToTransform` _returnvalue_4) "Undefined" "OverrideRootScale" null null))
          (bind _returnvalue_6 (`self.GetComponentByClass` _returnvalue_5 "/Script/Engine.StaticMeshComponent"))
          (`SceneComponent.SetMobility` _returnvalue_6 "Movable")
          (`PrimitiveComponent.SetSimulatePhysics` _returnvalue_6 true)
          (set `ActorComponent.ComponentTags` (`|MakeArray` "None" :!type "Name") (`self.GetComponentByClass` _returnvalue_5 "/Script/Engine.SceneComponent"))
          (`PhysicsHandleComponent.GrabComponentAtLocationWithRotation` :`self` _physicshandle :`Component` _returnvalue_6 :`Location` _returnvalue_4)
          (else
            (`PhysicsHandleComponent.GrabComponentAtLocationWithRotation` :`self` _physicshandle :`Component` _hitcomponent :`Location` _returnvalue_4)))
        (`PhysicsHandleComponent.SetTargetLocationAndRotation` _physicshandle (+ _returnvalue (* _returnvalue_2 130.0)) (`SceneComponent.K2_GetComponentRotation` _fpcamera) :!label _label_2))))
  (:`Released`
    (`PhysicsHandleComponent.ReleaseComponent` (`self.PhysicsHandle`))))

(event `InputAxis|Grabbing`
  (params (AxisValue :type "Float (single-precision)"))
  (goto _label_2))

(fn `UserConstructionScript`)