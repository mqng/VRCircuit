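; XOR logic gate actor that players wire up with Cable actors to combine two signals.
; A Cable overlapping either input trigger snaps its cable end to that input, which is tagged Connected, and the trigger is destroyed.
; Each Tick it reads the connected cables' OutputState and, once both inputs are connected, sets its own OutputState to their XOR.
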(event `self.ReceiveTick`
  (params (DeltaSeconds :type "Float (single-precision)"))
  (if (`ActorComponent.ComponentHasTag` (`self.Input_1`) "Connected")
    (set `self.Input1State` (`/Game/Blueprints/Cable.OutputState` (`self.Cable1`)))
    (if (`ActorComponent.ComponentHasTag` (`self.Input_2`) "Connected")
      (bind _output_get (set `self.Input2State` (`/Game/Blueprints/Cable.OutputState` (`self.Cable2`))))
      (set `self.OutputState` (xor _output_get (`self.Input1State`))))))

(event `self.InputTrigger1.OnComponentBeginOverlap`
  (params (OverlappedComponent :type "PrimitiveComponent Object Reference") (OtherActor :type "Actor Object Reference") (OtherComp :type "PrimitiveComponent Object Reference") (OtherBodyIndex :type Integer) (bFromSweep :type Boolean) (SweepResult :type "HitResult Structure (by ref)"))
  (bind _input_1 (`self.Input_1`))
  (bind _ascable (cast `/Game/Blueprints/Cable` OtherActor))
  (set `self.Cable1` _ascable)
  (if (not (`ActorComponent.ComponentHasTag` _input_1 "Connected"))
    (`CableComponent.SetAttachEndToComponent` (`/Game/Blueprints/Cable.Cable` _ascable) _input_1 "None")
    (set `ActorComponent.ComponentTags` (`|MakeArray` "Connected" :!type "Name") _input_1)
    (`ActorComponent.K2_DestroyComponent` (`self.InputTrigger1`))))

(event `self.InputTrigger2.OnComponentBeginOverlap`
  (params (OverlappedComponent :type "PrimitiveComponent Object Reference") (OtherActor :type "Actor Object Reference") (OtherComp :type "PrimitiveComponent Object Reference") (OtherBodyIndex :type Integer) (bFromSweep :type Boolean) (SweepResult :type "HitResult Structure (by ref)"))
  (bind _input_2 (`self.Input_2`))
  (bind _ascable (cast `/Game/Blueprints/Cable` OtherActor))
  (set `self.Cable2` _ascable)
  (if (not (`ActorComponent.ComponentHasTag` _input_2 "Connected"))
    (`CableComponent.SetAttachEndToComponent` (`/Game/Blueprints/Cable.Cable` _ascable) _input_2 "None")
    (set `ActorComponent.ComponentTags` (`|MakeArray` "Connected" :!type "Name") _input_2)
    (`ActorComponent.K2_DestroyComponent` (`self.InputTrigger2`))))

(fn `UserConstructionScript`)