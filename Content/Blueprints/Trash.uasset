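; Trash actor for VR that disposes of objects entering its box trigger while a pawn is holding something.
; On overlap, it searches all VRPawns for the first whose PhysicsHandle has a grabbed component and teleports that component to a fixed relative offset.
; It then adds a Niagara effect, plays a sound and, after a short delay, destroys the overlapping actor, without checking that it is the held object.
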(event `self.Box.OnComponentBeginOverlap`
  (params (OverlappedComponent :type "PrimitiveComponent Object Reference") (OtherActor :type "Actor Object Reference") (OtherComp :type "PrimitiveComponent Object Reference") (OtherBodyIndex :type Integer) (bFromSweep :type Boolean) (SweepResult :type "HitResult Structure (by ref)"))
  (bind _outactors (`GameplayStatics.GetAllActorsOfClass` "/Game/Blueprints/VRPawn.VRPawn_C"))
  (for _array_element _outactors
    (bind _returnvalue (`PhysicsHandleComponent.GetGrabbedComponent` (`/Game/Blueprints/VRPawn.PhysicsHandle` _array_element)))
    (if (`KismetSystemLibrary.IsValidClass` (`GameplayStatics.GetObjectClass` _returnvalue))
      (`SceneComponent.K2_SetRelativeTransform` _returnvalue (`KismetMathLibrary.MakeTransform` (0.0 0.0 500.0)) false true)
      (`AddComponent|NODE_AddNiagaraComponent-2`)
      (`GameplayStatics.PlaySoundAtLocation` "/Engine/EditorSounds/GamePreview/EndPlayInEditor.EndPlayInEditor" (0.0 0.0 0.0) (struct) 1.0 1.0 0.0 null null null)
      (`KismetSystemLibrary.Delay` 0.5)
      (`self.K2_DestroyActor` OtherActor)
      (break))))

(fn `UserConstructionScript`)